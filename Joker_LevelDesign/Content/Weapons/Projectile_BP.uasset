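; Projectile actor that detonates explosive barrels it touches.
; When its sphere overlaps an explosive barrel, it spawns an explosion particle, a Collision actor and a Force actor at the barrel's location, plays an explosion sound, then destroys the barrel.
; Overlaps with anything else are ignored, and the projectile itself is not destroyed by this graph.
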(event OnComponentBeginOverlap(Sphere)
  (params (OverlappedComponent :type Primitive%20Component%20Object%20Reference) (OtherActor :type Actor%20Object%20Reference) (OtherComp :type Primitive%20Component%20Object%20Reference) (OtherBodyIndex :type Integer) (bFromSweep :type Boolean) (SweepResult :type Hit%20Result%20Structure%20%28by%20ref%29))
  (bind _asexplosivebarrel (Utilities|Casting|CastToexplosivebarrel OtherActor))
  (Variables|Default|SetAs%20Explosivebarrel _asexplosivebarrel)
  (Effects|SpawnEmitteratLocation "/Game/StarterContent/Particles/P_Explosion.P_Explosion" (Transformation|GetWorldLocation (Variables|/Script/Engine.Actor|GetRootComponent (Variables|Default|GetAs%20Explosivebarrel))) "0, 0, 0" "4.000000,4.000000,4.000000")
  (Game|SpawnActorfromClass "/Game/Weapons/ExplosiveBarrel/collision.collision_C" (Math|Transform|MakeTransform (Transformation|GetWorldLocation (Variables|/Script/Engine.Actor|GetRootComponent (Variables|Default|GetAs%20Explosivebarrel))) "0, 0, 0" "1,1,1") "Undefined" 0 0)
  (Game|SpawnActorfromClass "/Game/Weapons/ExplosiveBarrel/force.force_C" (Math|Transform|MakeTransform (Transformation|GetWorldLocation (Variables|/Script/Engine.Actor|GetRootComponent (Variables|Default|GetAs%20Explosivebarrel))) "0, 0, 0" "1.000000,1,1") "Undefined" 0 0)
  (Audio|PlaySoundatLocation "/Game/StarterContent/Audio/Explosion01.Explosion01" (Transformation|GetWorldLocation (Variables|/Script/Engine.Actor|GetRootComponent (Variables|Default|GetAs%20Explosivebarrel))) "0, 0, 0" 0.8 1.0 0.0 0 0 0)
  (Actor|DestroyActor (Variables|Default|GetAs%20Explosivebarrel)))

(event EventBeginPlay)

(event Collision|EventActorBeginOverlap
  (params (OtherActor :type Actor%20Object%20Reference)))

(event EventTick
  (params (DeltaSeconds :type Float%20%28single-precision%29)))

(fn ConstructionScript)