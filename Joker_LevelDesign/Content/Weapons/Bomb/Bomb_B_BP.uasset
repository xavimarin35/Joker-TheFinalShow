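; Bomb site B actor that lets the JokerCharacter plant a bomb by pressing Interaction inside its Box trigger.
; Box overlap begin and end toggle the actor's input for the first player controller.
; A one-shot press disables player input, plays a montage and 2D sound, then after a delay restores input and sets IsBPlanted on the character.
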(event OnComponentBeginOverlap(Box)
  (params (OverlappedComponent :type Primitive%20Component%20Object%20Reference) (OtherActor :type Actor%20Object%20Reference) (OtherComp :type Primitive%20Component%20Object%20Reference) (OtherBodyIndex :type Integer) (bFromSweep :type Boolean) (SweepResult :type Hit%20Result%20Structure%20%28by%20ref%29))
  (Utilities|Casting|CastToJokerCharacter OtherActor)
  (Input|EnableInput (Game|GetPlayerController 0)))

(event OnComponentEndOverlap(Box)
  (params (OverlappedComponent :type Primitive%20Component%20Object%20Reference) (OtherActor :type Actor%20Object%20Reference) (OtherComp :type Primitive%20Component%20Object%20Reference) (OtherBodyIndex :type Integer))
  (Utilities|Casting|CastToJokerCharacter OtherActor)
  (Input|DisableInput (Game|GetPlayerController 0)))

(event Input|ActionEvents|InputActionInteraction
  (params (Key :type Key%20Structure :default "None"))
  (:Pressed
    (Utilities|FlowControl|DoOnce false
      (:Completed
        (Input|DisableInput (Game|GetPlayerCharacter 0) (Game|GetPlayerController 0))
        (bind _asjoker_character (Utilities|Casting|CastToJokerCharacter (Game|GetPlayerCharacter 0)))
        (Animation|PlayAnimMontage _asjoker_character "/Game/Weapons/Bomb/Animations/Opening_Anim_Montage.Opening_Anim_Montage" 1.0 "None")
        (Audio|PlaySound2D 0 1.0 1.0 0.0 0 0)
        (Utilities|FlowControl|Delay 5.0)
        (Input|EnableInput (Game|GetPlayerCharacter 0) (Game|GetPlayerController 0))
        (Variables|/Game/ThirdPersonBP/Blueprints/JokerCharacter.JokerCharacter_C|SetIsBPlanted? _asjoker_character true)))))

(fn ConstructionScript)