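; A door Blueprint that the player can kick open once when standing in its trigger box.
; Box overlap toggles actor input and a prompt widget, which no longer appears after Interaction is released and clears IsOpen.
; Pressing Interaction locks player input, snaps the character to the SkeletalMesh transform and plays a kick montage while a timeline swings the door.
; A delayed one-shot from the timeline plays a sound and restores input.
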(event OnComponentBeginOverlap(Box)
  (params (OverlappedComponent :type Primitive%20Component%20Object%20Reference) (OtherActor :type Actor%20Object%20Reference) (OtherComp :type Primitive%20Component%20Object%20Reference) (OtherBodyIndex :type Integer) (bFromSweep :type Boolean) (SweepResult :type Hit%20Result%20Structure%20%28by%20ref%29))
  (Utilities|Casting|CastToThirdPersonCharacter OtherActor)
  (Input|EnableInput (Game|GetPlayerController 0))
  (if (Variables|Default|GetIsOpen?)
    (bind _returnvalue (UserInterface|CreateWidget "/Game/OtherAnimations/KickDoorWB.KickDoorWB_C"))
    (UserInterface|Viewport|AddtoViewport _returnvalue 0)))

(event OnComponentEndOverlap(Box)
  (params (OverlappedComponent :type Primitive%20Component%20Object%20Reference) (OtherActor :type Actor%20Object%20Reference) (OtherComp :type Primitive%20Component%20Object%20Reference) (OtherBodyIndex :type Integer))
  (Utilities|Casting|CastToThirdPersonCharacter OtherActor)
  (Input|DisableInput (Game|GetPlayerController 0))
  (Widget|RemovefromParent (stale OnComponentBeginOverlap(Box) _returnvalue)))

(event Input|ActionEvents|InputActionInteraction
  (params (Key :type Key%20Structure :default "None"))
  (:Pressed
    (Utilities|FlowControl|DoOnce false
      (:Completed
        (Input|DisableInput (Game|GetPlayerCharacter 0) (Game|GetPlayerController 0))
        (bind _asthird_person_character (Utilities|Casting|CastToThirdPersonCharacter (Game|GetPlayerCharacter 0)))
        (Transformation|SetActorTransform _asthird_person_character (Transformation|GetWorldTransform (Variables|Default|GetSkeletalMesh)))
        (Animation|PlayAnimMontage _asthird_person_character "/Game/OtherAnimations/Kicking__1__Anim_Montage.Kicking__1__Anim_Montage" 1.0 "None")
        (bind _door_kick_track (Timeline|Kick%20Open%20Door Play)
          (:Update
            (Transformation|SetRelativeRotation (Variables|Default|GetDoor) (Math|Rotator|MakeRotator 0.0 0.0 (Math|Float|Lerp 0.0 -1e+02 _door_kick_track)) false false)
            (Utilities|FlowControl|DoOnce false
              (:Completed
                (Utilities|FlowControl|Delay 1.0)
                (Audio|PlaySound2D "/Game/Sounds/AK47_S_Cue.AK47_S_Cue" 1.0 1.0 0.0 0 0 false)
                (Input|EnableInput (Game|GetPlayerCharacter 0) (Game|GetPlayerController 0)))))))))
  (:Released
    (Widget|RemovefromParent (stale OnComponentBeginOverlap(Box) _returnvalue))
    (Variables|Default|SetIsOpen? false)))

(fn ConstructionScript)